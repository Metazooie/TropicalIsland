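; Spline-based cave actor that builds a cave out of repeated mesh segments along its spline in the construction script.
; Section length is a base value scaled by the actor's X scale, and BuildSpline adds one CaveMesh01 spline mesh component per whole section, leaving any remainder uncovered.
; Each segment takes local-space positions and tangents from the spline, with tangents clamped to section length.
; The event graph has no active logic.
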(fn `BuildSpline`
  (bind _spline (`self.Spline`))
  (bind _section_lengh (`self.Section Lengh`))
  (for _index (range (`KismetMathLibrary.FFloor` (/ (`SplineComponent.GetSplineLength` (`self.Spline`)) (`self.Section Lengh`))))
    (bind _returnvalue (`AddComponent|NODE_AddSplineMeshComponent-0`))
    (`StaticMeshComponent.SetStaticMesh` _returnvalue (`self.CaveMesh01`))
    (`SplineMeshComponent.SetForwardAxis` _returnvalue "X" true)
    (bind _returnvalue_2 (* _index (`self.Section Lengh`)))
    (bind _returnvalue_3 (* (+ _index 1) (`self.Section Lengh`)))
    (`SplineMeshComponent.SetStartAndEnd` _returnvalue (`SplineComponent.GetLocationAtDistanceAlongSpline` _spline _returnvalue_2 "Local") (`KismetMathLibrary.ClampVectorSize` (`SplineComponent.GetTangentAtDistanceAlongSpline` _spline _returnvalue_2 "Local") 0.0 _section_lengh) (`SplineComponent.GetLocationAtDistanceAlongSpline` _spline _returnvalue_3 "Local") (`KismetMathLibrary.ClampVectorSize` (`SplineComponent.GetTangentAtDistanceAlongSpline` _spline _returnvalue_3 "Local") 0.0 _section_lengh) true)))

(fn `UserConstructionScript`
  (bind _returnvalue_x (`KismetMathLibrary.BreakVector` (`self.GetActorScale3D`)))
  (set `self.Section Lengh` (* 500 _returnvalue_x))
  (`self.BuildSpline`))