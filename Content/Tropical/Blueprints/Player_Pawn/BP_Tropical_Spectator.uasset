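; BP_Tropical_Spectator is the spectator player pawn for the Tropical content, which sets up the session and shows a rain control UI.
; On BeginPlay it applies rendering and performance console commands for sharpening, frame cap, streaming pool, shadow filtering and DLSS.
; It then enables input with a visible cursor in Game and UI mode and adds the BPU_RainControl widget to the viewport.
; Leftover nodes mapping Raininess to two Niagara RainAmount variables are disconnected and never run.
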(event `self.ReceiveTick`
  (params (DeltaSeconds :type "Float (single-precision)")))

(event `self.ReceiveBeginPlay`
  (bind _returnvalue (`GameplayStatics.GetPlayerController` 0))
  (`KismetSystemLibrary.ExecuteConsoleCommand` "r.Tonemapper.Sharpen 2" null)
  (`KismetSystemLibrary.ExecuteConsoleCommand` "t.MaxFPS 60" null)
  (`KismetSystemLibrary.ExecuteConsoleCommand` "r.Streaming.PoolSize 2048" null)
  (`KismetSystemLibrary.ExecuteConsoleCommand` "r.Shadow.FilterMethod 1" null)
  (`KismetSystemLibrary.ExecuteConsoleCommand` "r.NGX.DLSS.Enable 1" null)
  (`KismetSystemLibrary.ExecuteConsoleCommand` "r.NGX.DLSS.Quality Perfomance" null)
  (`self.EnableInput` _returnvalue)
  (set `PlayerController.bShowMouseCursor` true _returnvalue)
  (`WidgetBlueprintLibrary.SetInputMode_GameAndUIEx` _returnvalue null)
  (bind _returnvalue_2 (`|CreateWidget` "/Game/Tropical/Blueprints/RainSystem/Blueprints/RainControl/BPU_RainControl.BPU_RainControl_C" _returnvalue))
  (`UserWidget.AddToViewport` _returnvalue_2 0))

(fn `UserConstructionScript`)